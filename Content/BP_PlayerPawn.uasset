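; Player pawn with a spring-arm camera that flies or moves by Enhanced Input and can trigger Mass entity spawning.
; Move input pushes along the control rotation's forward and right vectors, while look input drives controller yaw and pitch.
; Zoom inputs step the spring arm length within clamped limits on both triggered and ongoing events.
; The spawn action executes a MassSpawner.
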(event `EnhancedInput|/Game/input/Actions/IA_Move`
  (params (ActionValue :type "Vector2D Structure") (ElapsedSeconds :type "Float (double-precision)") (TriggeredSeconds :type "Float (double-precision)") (InputAction :type "InputAction Object Reference" :default "/Game/input/Actions/IA_Move.IA_Move"))
  (:`Triggered`
    (`self.AddMovementInput` (* (`KismetMathLibrary.GetRightVector` (`self.GetControlRotation`)) ActionValue_X))
    (`self.AddMovementInput` (* (`KismetMathLibrary.GetForwardVector` (`self.GetControlRotation`)) ActionValue_Y))))

(event `EnhancedInput|/Game/input/Actions/IA_Look`
  (params (ActionValue :type "Vector2D Structure") (ElapsedSeconds :type "Float (double-precision)") (TriggeredSeconds :type "Float (double-precision)") (InputAction :type "InputAction Object Reference" :default "/Game/input/Actions/IA_Look.IA_Look"))
  (:`Triggered`
    (`self.AddControllerYawInput` ActionValue_X)
    (`self.AddControllerPitchInput` ActionValue_Y)))

(event `EnhancedInput|/Game/input/Actions/IA_ZoomOut`
  (params (ActionValue :type "Vector2D Structure") (ElapsedSeconds :type "Float (double-precision)") (TriggeredSeconds :type "Float (double-precision)") (InputAction :type "InputAction Object Reference" :default "/Game/input/Actions/IA_ZoomOut.IA_ZoomOut"))
  (bind _springarm (`self.SpringArm`))
  (:`Triggered`
    (set `SpringArmComponent.TargetArmLength` (`KismetMathLibrary.FClamp` (+ (`SpringArmComponent.TargetArmLength` _springarm) 100.0) 500.0 3000.0) _springarm :!label _label))
  (:`Ongoing`
    (goto _label)))

(event `EnhancedInput|/Game/input/Actions/IA_ZoomIn`
  (params (ActionValue :type "Vector2D Structure") (ElapsedSeconds :type "Float (double-precision)") (TriggeredSeconds :type "Float (double-precision)") (InputAction :type "InputAction Object Reference" :default "/Game/input/Actions/IA_ZoomIn.IA_ZoomIn"))
  (bind _springarm (`self.SpringArm`))
  (:`Triggered`
    (set `SpringArmComponent.TargetArmLength` (`KismetMathLibrary.FClamp` (- (`SpringArmComponent.TargetArmLength` _springarm) 100.0) 500.0 3000.0) _springarm :!label _label_2))
  (:`Ongoing`
    (goto _label_2)))

(event `EnhancedInput|/Game/input/Actions/IA_Spawn`
  (params (ActionValue :type Boolean) (ElapsedSeconds :type "Float (double-precision)") (TriggeredSeconds :type "Float (double-precision)") (InputAction :type "InputAction Object Reference" :default "/Game/input/Actions/IA_Spawn.IA_Spawn"))
  (:`Triggered`
    (`MassSpawnerComponent.Execute` (`self.MassSpawner`))))

(fn `UserConstructionScript`)